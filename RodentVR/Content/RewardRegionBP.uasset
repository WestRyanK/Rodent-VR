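; Reward region actor that reacts when something overlaps its Collision component, driving a reward dispenser and a tone generator.
; On begin overlap it signals OnRewardRegionEnter with its RegionId, dispenses a timed reward on the configured device and plays a timed synth tone, each behind an enable flag.
; On end overlap it signals -1, stops the tone and, if dispensing is enabled, stops rewards.
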(event `self.Collision.OnComponentBeginOverlap`
  (params (OverlappedComponent :type "PrimitiveComponent Object Reference") (OtherActor :type "Actor Object Reference") (OtherComp :type "PrimitiveComponent Object Reference") (OtherBodyIndex :type Integer) (bFromSweep :type Boolean) (SweepResult :type "HitResult Structure (by ref)"))
  (`self.OnRewardRegionEnter` (`self.RegionId`))
  (`self.HandleRewardDispenser` true)
  (`self.HandleToneGenerator` true))

(event `self.Collision.OnComponentEndOverlap`
  (params (OverlappedComponent :type "PrimitiveComponent Object Reference") (OtherActor :type "Actor Object Reference") (OtherComp :type "PrimitiveComponent Object Reference") (OtherBodyIndex :type Integer))
  (`self.OnRewardRegionEnter` -1)
  (`self.HandleRewardDispenser` false)
  (`self.HandleToneGenerator` false))

(fn `HandleRewardDispenser`
  (params (IsBeginOverlap :type Boolean))
  (bind _rewarddispenser (`self.RewardDispenser`))
  (bind _isrewarddispensingenabled (`self.IsRewardDispensingEnabled`))
  (if IsBeginOverlap
    (if _isrewarddispensingenabled
      (`/Game/RewardDispenser.DispenseReward` _rewarddispenser (`self.RewardDeviceId`) (`self.RewardDurationSec`)))
    (elif _isrewarddispensingenabled
      (`/Game/RewardDispenser.StopDispensingRewards` _rewarddispenser)))
  (return))

(fn `HandleToneGenerator`
  (params (IsBeginOverlap :type Boolean))
  (if (and IsBeginOverlap (`self.IsToneEnabled`))
    (`ToneGenerator.StartTimedSynth` (`self.ToneGenerator`) (`self.ToneDurationSec`) (`self.TonePitchHz`) (`self.ToneVolumeMultiplier`))
    (else
      (`SynthComponent.Stop` (`self.ToneGenerator`))))
  (return))

(fn `UserConstructionScript`)