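; Game mode for the RodentVR simulator that prepares a session and clears the spawned maze on end play.
; On begin play it caches the game instance, sets game-only input and checks NI-DAQ settings.
; If NI-DAQ and its warning are enabled, a dialog offers to start the services or returns to the main menu.
; NI-DAQ initialization, maze loading and graphics setup are present but unwired.
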(event `self.ReceiveBeginPlay`
  (bind _asrodent_vrgame_instance (cast `RodentVRGameInstance` (`GameplayStatics.GetGameInstance`)))
  (set `self.Game Instance` _asrodent_vrgame_instance)
  (`WidgetBlueprintLibrary.SetInputMode_GameOnly` (`GameplayStatics.GetPlayerController` 0))
  (`self.EnsureNIDAQServicesEnabled`))

(event `self.ReceiveEndPlay`
  (params (EndPlayReason :type "EEndPlayReason Enum" :default "Destroyed"))
  (`MazeSpawner.ClearSpawnedMaze` self))

(fn `EnsureNIDAQServicesEnabled`
  (if (`RodentVRSettings.IsNidaqEnabled` (`RodentVRGameInstance.RodentVRSettings` (`self.Game Instance`)))
    (`NIDAQServiceManager.GetAreAllNidaqServicesRunning`)
    (if (`RodentVRSettings.ShouldWarnIfNidaqServicesDisabled` (`RodentVRGameInstance.RodentVRSettings` (`self.Game Instance`)))
      (bind _returnvalue (`TinyFileDialogsLib.ShowMessageBox` "Restart NIDAQ Services" "NIDAQ services appear to be stopped, which could potentially cause RodentVR to freeze. Would you like to try starting them?" "YESNOCANCEL" "INFO"))
      (switch `int` _returnvalue
        (:`Default`
          (`RodentVRGameInstance.GoToPage` (`self.Game Instance`) "MAINMENU" :!label _label))
        (:`0`
          (goto _label))
        (:`1`
          (`TinyFileDialogsLib.ShowMessageBox` "Starting Services" "Starting NI DAQ Services... This may take a couple minutes" "OK" "INFO")
          (`NIDAQServiceManager.StartAllNidaqServices`))))))

(fn `UserConstructionScript`)